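; Player-controlled robot character Blueprint that adds a toggleable flying mode.
; The 1 key drives a FlipFlop that switches the CharacterMovement mode between Flying and Walking.
; The MoveFlying axis adds movement input along the actor's up vector for vertical control, without checking the current mode.
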(event EventBeginPlay
  (|CallParentFunction))

(event Collision|EventActorBeginOverlap
  (params (OtherActor :type Actor%20Object%20Reference))
  (|CallParentFunction OtherActor))

(event EventTick
  (params (DeltaSeconds :type Float%20%28single-precision%29))
  (|CallParentFunction DeltaSeconds))

(event Input|AxisEvents|InputAxisMoveFlying
  (params (AxisValue :type Float%20%28single-precision%29))
  ;[1 1 1] Flying
  (Pawn|Input|AddMovementInput (Transformation|GetActorUpVector) AxisValue false))

(event Input|KeyboardEvents|1
  (params (Key :type Key%20Structure))
  (bind _charactermovement (Variables|Character|GetCharacterMovement))
  ;[1 1 1] Flying
  (:Pressed
    (Utilities|FlowControl|FlipFlop
      (:A
        (Pawn|Components|CharacterMovement|SetMovementMode _charactermovement "MOVE_Flying" 0))
      (:B
        (Pawn|Components|CharacterMovement|SetMovementMode _charactermovement "MOVE_Walking" 0)))))

(fn ConstructionScript
  (|CallParentFunction))